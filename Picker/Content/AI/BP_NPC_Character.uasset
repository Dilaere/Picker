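; NPC character that feeds its AI blackboard the data to flee whenever the player's backpack holds an item.
; On BeginPlay it caches the blackboard from BP_NPC_Controller and the player's BackpackComponent.
; A backpack change event, unbound on EndPlay, updates ShouldRunAway from HasItem.
; Tick continually sets AwayPoint a fixed distance from the NPC, directly away from the player.
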(event `self.ReceiveBeginPlay`
  (bind _asbp_npc_controller (cast `/Game/AI/BP_NPC_Controller` (`self.GetController`)))
  (set `self.BlackboardComponent` (`AIController.Blackboard` _asbp_npc_controller))
  (set `self.PlayerBackpackComponent` (`self.GetComponentByClass` (`GameplayStatics.GetPlayerCharacter` 0) "/Script/Picker.BackpackComponent"))
  (add `BackpackComponent.OnBackpackChanged` (`self.PlayerBackpackComponent`) (delegate `OnPlayerBackpackChanged`)))

(event `self.ReceiveEndPlay`
  (params (EndPlayReason :type "EEndPlayReason Enum" :default "Destroyed"))
  (`|ExecutionSequence`
    (:`then_0`
      (bind _playerbackpackcomponent (`self.PlayerBackpackComponent`)
        (:`then`
          (remove `BackpackComponent.OnBackpackChanged` _playerbackpackcomponent (delegate `OnPlayerBackpackChanged`)))
        (:`else`)))
    (:`then_1`
      (`parent.ReceiveEndPlay` EndPlayReason))))

(event `OnPlayerBackpackChanged`
  (`BlackboardComponent.SetValueAsBool` (`self.BlackboardComponent`) (`KismetStringLibrary.Conv_StringToName` "ShouldRunAway") (`BackpackComponent.HasItem` (`self.PlayerBackpackComponent`))))

(event `self.ReceiveTick`
  (params (DeltaSeconds :type "Float (single-precision)"))
  (bind _returnvalue (`self.K2_GetActorLocation`))
  (bind _blackboardcomponent (`self.BlackboardComponent`)
    (:`then`
      (`BlackboardComponent.SetValueAsVector` _blackboardcomponent (`KismetStringLibrary.Conv_StringToName` "AwayPoint") (+ _returnvalue (* (`KismetMathLibrary.GetDirectionUnitVector` (`self.K2_GetActorLocation` (`GameplayStatics.GetPlayerCharacter` 0)) _returnvalue) 300))))
    (:`else`)))

(fn `UserConstructionScript`)